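; Player character that drives a 2048-style number cube game from the arrow keys.
; On BeginPlay it requests two cubes, each from a randomly picked BP_CubeSpawner out of sixteen.
; Each key press calls the matching directional move on every BP_NumberCube, then after a short Delay spawns one or two new cubes.
; A failed spawn loops back through a short Delay to retry another random spawner.
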(event `self.ReceiveBeginPlay`
  (`self.Start`))

(event `Start`
  (for _ (range 2)
    (bind _outactors (`GameplayStatics.GetAllActorsOfClass` "/Game/Blueprint/BP_CubeSpawner.BP_CubeSpawner_C" :!label _label))
    (bind _success (`/Game/Blueprint/BP_CubeSpawner.SpawnCube` (`|GetArrayItem` _outactors (`KismetMathLibrary.RandomInteger` 16))))
    (if (not _success)
      (`KismetSystemLibrary.Delay` 0.01)
      (goto _label))))

(event `Key|Up`
  (params (Key :type "Key Structure"))
  (:`Pressed`
    (bind _outactors (`GameplayStatics.GetAllActorsOfClass` "/Game/Blueprint/BP_NumberCube.BP_NumberCube_C"))
    (for _array_element _outactors
      (`/Engine/EditorBlueprintResources/StandardMacros.IsValid` _array_element
        (:`Is Valid`
          (`/Game/Blueprint/BP_NumberCube.MoveUp` _array_element)
          (`KismetSystemLibrary.Delay` 0.01 :!label _label_2)
          (`self.SpawnCube`))))))

(event `Key|Down`
  (params (Key :type "Key Structure"))
  (:`Pressed`
    (bind _outactors (`GameplayStatics.GetAllActorsOfClass` "/Game/Blueprint/BP_NumberCube.BP_NumberCube_C"))
    (for _array_element _outactors
      (`/Engine/EditorBlueprintResources/StandardMacros.IsValid` _array_element
        (:`Is Valid`
          (`/Game/Blueprint/BP_NumberCube.MoveDown` _array_element)
          (goto _label_2))))))

(event `Key|Right`
  (params (Key :type "Key Structure"))
  (:`Pressed`
    (bind _outactors (`GameplayStatics.GetAllActorsOfClass` "/Game/Blueprint/BP_NumberCube.BP_NumberCube_C"))
    (for _array_element _outactors
      (`/Engine/EditorBlueprintResources/StandardMacros.IsValid` _array_element
        (:`Is Valid`
          (`/Game/Blueprint/BP_NumberCube.MoveRight` _array_element)
          (goto _label_2))))))

(event `Key|Left`
  (params (Key :type "Key Structure"))
  (:`Pressed`
    (bind _outactors (`GameplayStatics.GetAllActorsOfClass` "/Game/Blueprint/BP_NumberCube.BP_NumberCube_C"))
    (for _array_element _outactors
      (`/Engine/EditorBlueprintResources/StandardMacros.IsValid` _array_element
        (:`Is Valid`
          (`/Game/Blueprint/BP_NumberCube.MoveLeft` _array_element)
          (goto _label_2))))))

(event `SpawnCube`
  (for _ (range (+ (`KismetMathLibrary.RandomIntegerInRange` 0 1) 1))
    (bind _outactors (`GameplayStatics.GetAllActorsOfClass` "/Game/Blueprint/BP_CubeSpawner.BP_CubeSpawner_C" :!label _label_3))
    (bind _success (`/Game/Blueprint/BP_CubeSpawner.SpawnCube` (`|GetArrayItem` _outactors (`KismetMathLibrary.RandomInteger` 16))))
    (if (not _success)
      (`KismetSystemLibrary.Delay` 0.01)
      (goto _label_3))))

(fn `UserConstructionScript`)