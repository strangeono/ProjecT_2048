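; Numbered tile actor for a 2048-style sliding puzzle, showing its value through a W_NumberWidget.
; Each Move function probes one grid step along the cube's axes by spawning a temporary BP_Checker at the trace end.
; It steps into free cells, merges with an equal-numbered cube by doubling and destroying it, and stops at edges or different numbers.
; Moves recurse, so a cube keeps sliding and can chain several merges in one move.
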(event `UpdateNumberText`
  (`TextBlock.SetText` (`/Game/Blueprint/W_NumberWidget.NumberText` (stale `self.ReceiveBeginPlay` _asw_number_widget)) (`KismetTextLibrary.Conv_IntToText` (`self.Number`)) :!label _label))

(event `self.ReceiveBeginPlay`
  (bind _asw_number_widget (cast `/Game/Blueprint/W_NumberWidget` (`WidgetComponent.GetWidget` (`self.Widget`))))
  (goto _label))

(fn `MoveDown`
  (bind _cube (`self.Cube`))
  (bind _returnvalue (`SceneComponent.K2_GetComponentLocation` _cube))
  (bind _outhit (`KismetSystemLibrary.LineTraceSingle` :`Start` _returnvalue :`End` (+ _returnvalue (* (`KismetMathLibrary.GetUpVector` (`SceneComponent.K2_GetComponentRotation` _cube)) -80.0)) :`TraceChannel` "TraceTypeQuery1" :`DrawDebugType` "Persistent"))
  (bind (_bblockinghit _binitialoverlap _time _distance _location _impactpoint _normal _impactnormal _physmat _hitactor _hitcomponent _hitbonename _bonename _hititem _elementindex _faceindex _tracestart _traceend) (`GameplayStatics.BreakHitResult` _outhit))
  (bind _returnvalue_2 (`|SpawnActorFromClass` "/Game/Blueprint/BP_Checker.BP_Checker_C" (`KismetMathLibrary.MakeTransform` _traceend) "Undefined" "MultiplyWithRoot" null null))
  (bind _success (`/Game/Blueprint/BP_Checker.AreWeOverlapping` _returnvalue_2))
  (if _success
    (bind _asbp_number_cube (`/Game/Blueprint/BP_Checker.WhoAreWeOverlapping` _returnvalue_2))
    (if (== (`/Game/Blueprint/BP_NumberCube.Number` _asbp_number_cube) (`self.Number`))
      (set `self.Number` (* (`self.Number`) 2))
      (`self.K2_DestroyActor` _returnvalue_2)
      (`SceneComponent.K2_SetWorldLocation` (`self.DefaultSceneRoot`) _traceend false false)
      (`self.K2_DestroyActor` _asbp_number_cube)
      (`self.UpdateNumberText`)
      (`self.MoveDown`)
      (return)
      (else
        (`self.K2_DestroyActor` _returnvalue_2)
        (return)))
    (else
      (bind _success_2 (`/Game/Blueprint/BP_Checker.AreWeAtTheEnd` _returnvalue_2))
      (if _success_2
        (`self.K2_DestroyActor` _returnvalue_2)
        (return)
        (else
          (`SceneComponent.K2_SetWorldLocation` (`self.DefaultSceneRoot`) _traceend false false)
          (`self.K2_DestroyActor` _returnvalue_2)
          (`self.MoveDown`)
          (return))))))

(fn `MoveLeft`
  (bind _cube (`self.Cube`))
  (bind _returnvalue (`SceneComponent.K2_GetComponentLocation` _cube))
  (bind _outhit (`KismetSystemLibrary.LineTraceSingle` :`Start` _returnvalue :`End` (+ _returnvalue (* (`KismetMathLibrary.GetRightVector` (`SceneComponent.K2_GetComponentRotation` _cube)) 80.0)) :`TraceChannel` "TraceTypeQuery1" :`DrawDebugType` "Persistent"))
  (bind (_bblockinghit _binitialoverlap _time _distance _location _impactpoint _normal _impactnormal _physmat _hitactor _hitcomponent _hitbonename _bonename _hititem _elementindex _faceindex _tracestart _traceend) (`GameplayStatics.BreakHitResult` _outhit))
  (bind _returnvalue_2 (`|SpawnActorFromClass` "/Game/Blueprint/BP_Checker.BP_Checker_C" (`KismetMathLibrary.MakeTransform` _traceend) "Undefined" "MultiplyWithRoot" null null))
  (bind _success (`/Game/Blueprint/BP_Checker.AreWeOverlapping` _returnvalue_2))
  (if _success
    (bind _asbp_number_cube (`/Game/Blueprint/BP_Checker.WhoAreWeOverlapping` _returnvalue_2))
    (if (== (`/Game/Blueprint/BP_NumberCube.Number` _asbp_number_cube) (`self.Number`))
      (set `self.Number` (* (`self.Number`) 2))
      (`self.K2_DestroyActor` _returnvalue_2)
      (`SceneComponent.K2_SetWorldLocation` (`self.DefaultSceneRoot`) _traceend false false)
      (`self.K2_DestroyActor` _asbp_number_cube)
      (`self.UpdateNumberText`)
      (`self.MoveLeft`)
      (return)
      (else
        (`self.K2_DestroyActor` _returnvalue_2)
        (return)))
    (else
      (bind _success_2 (`/Game/Blueprint/BP_Checker.AreWeAtTheEnd` _returnvalue_2))
      (if _success_2
        (`self.K2_DestroyActor` _returnvalue_2)
        (return)
        (else
          (`SceneComponent.K2_SetWorldLocation` (`self.DefaultSceneRoot`) _traceend false false)
          (`self.K2_DestroyActor` _returnvalue_2)
          (`self.MoveLeft`)
          (return))))))

(fn `MoveRight`
  (bind _cube (`self.Cube`))
  (bind _returnvalue (`SceneComponent.K2_GetComponentLocation` _cube))
  (bind _outhit (`KismetSystemLibrary.LineTraceSingle` :`Start` _returnvalue :`End` (+ _returnvalue (* (`KismetMathLibrary.GetRightVector` (`SceneComponent.K2_GetComponentRotation` _cube)) -80.0)) :`TraceChannel` "TraceTypeQuery1" :`DrawDebugType` "Persistent"))
  (bind (_bblockinghit _binitialoverlap _time _distance _location _impactpoint _normal _impactnormal _physmat _hitactor _hitcomponent _hitbonename _bonename _hititem _elementindex _faceindex _tracestart _traceend) (`GameplayStatics.BreakHitResult` _outhit))
  (bind _returnvalue_2 (`|SpawnActorFromClass` "/Game/Blueprint/BP_Checker.BP_Checker_C" (`KismetMathLibrary.MakeTransform` _traceend) "Undefined" "MultiplyWithRoot" null null))
  (bind _success (`/Game/Blueprint/BP_Checker.AreWeOverlapping` _returnvalue_2))
  (if _success
    (bind _asbp_number_cube (`/Game/Blueprint/BP_Checker.WhoAreWeOverlapping` _returnvalue_2))
    (if (== (`/Game/Blueprint/BP_NumberCube.Number` _asbp_number_cube) (`self.Number`))
      (set `self.Number` (* (`self.Number`) 2))
      (`self.K2_DestroyActor` _returnvalue_2)
      (`SceneComponent.K2_SetWorldLocation` (`self.DefaultSceneRoot`) _traceend false false)
      (`self.K2_DestroyActor` _asbp_number_cube)
      (`self.UpdateNumberText`)
      (`self.MoveRight`)
      (return)
      (else
        (`self.K2_DestroyActor` _returnvalue_2)
        (return)))
    (else
      (bind _success_2 (`/Game/Blueprint/BP_Checker.AreWeAtTheEnd` _returnvalue_2))
      (if _success_2
        (`self.K2_DestroyActor` _returnvalue_2)
        (return)
        (else
          (`SceneComponent.K2_SetWorldLocation` (`self.DefaultSceneRoot`) _traceend false false)
          (`self.K2_DestroyActor` _returnvalue_2)
          (`self.MoveRight`)
          (return))))))

(fn `MoveUp`
  (bind _cube (`self.Cube`))
  (bind _returnvalue (`SceneComponent.K2_GetComponentLocation` _cube))
  (bind _outhit (`KismetSystemLibrary.LineTraceSingle` :`Start` _returnvalue :`End` (+ _returnvalue (* (`KismetMathLibrary.GetUpVector` (`SceneComponent.K2_GetComponentRotation` _cube)) 80.0)) :`TraceChannel` "TraceTypeQuery1" :`DrawDebugType` "Persistent"))
  (bind (_bblockinghit _binitialoverlap _time _distance _location _impactpoint _normal _impactnormal _physmat _hitactor _hitcomponent _hitbonename _bonename _hititem _elementindex _faceindex _tracestart _traceend) (`GameplayStatics.BreakHitResult` _outhit))
  (bind _returnvalue_2 (`|SpawnActorFromClass` "/Game/Blueprint/BP_Checker.BP_Checker_C" (`KismetMathLibrary.MakeTransform` _traceend) "Undefined" "MultiplyWithRoot" null null))
  (bind _success (`/Game/Blueprint/BP_Checker.AreWeOverlapping` _returnvalue_2))
  (if _success
    (bind _asbp_number_cube (`/Game/Blueprint/BP_Checker.WhoAreWeOverlapping` _returnvalue_2))
    (if (== (`/Game/Blueprint/BP_NumberCube.Number` _asbp_number_cube) (`self.Number`))
      (set `self.Number` (* (`self.Number`) 2))
      (`self.K2_DestroyActor` _returnvalue_2)
      (`SceneComponent.K2_SetWorldLocation` (`self.DefaultSceneRoot`) _traceend false false)
      (`self.K2_DestroyActor` _asbp_number_cube)
      (`self.UpdateNumberText`)
      (`self.MoveUp`)
      (return)
      (else
        (`self.K2_DestroyActor` _returnvalue_2)
        (return)))
    (else
      (bind _success_2 (`/Game/Blueprint/BP_Checker.AreWeAtTheEnd` _returnvalue_2))
      (if _success_2
        (`self.K2_DestroyActor` _returnvalue_2)
        (return)
        (else
          (`SceneComponent.K2_SetWorldLocation` (`self.DefaultSceneRoot`) _traceend false false)
          (`self.K2_DestroyActor` _returnvalue_2)
          (`self.MoveUp`)
          (return))))))

(fn `UserConstructionScript`)