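; BP_Checker is a probe actor that reports what occupies its Box component's space among number cubes and cube spawners.
; It exposes overlap queries for whether a BP_NumberCube is present and which one is first.
; A third query treats the absence of any overlapping BP_CubeSpawner as being "at the end".
; It has no active event logic, so it only answers when called.
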(fn `AreWeAtTheEnd`
  (returns (Success :type Boolean))
  (return (`KismetArrayLibrary.Array_IsEmpty` (`PrimitiveComponent.GetOverlappingActors` (`self.Box`) "/Game/Blueprint/BP_CubeSpawner.BP_CubeSpawner_C"))))

(fn `AreWeOverlapping`
  (returns (Success :type Boolean))
  (return (`KismetArrayLibrary.Array_IsNotEmpty` (`PrimitiveComponent.GetOverlappingActors` (`self.Box`) "/Game/Blueprint/BP_NumberCube.BP_NumberCube_C"))))

(fn `UserConstructionScript`)

(fn `WhoAreWeOverlapping`
  (returns (`AsBP Number Cube` :type "/Game/Blueprint/BP_NumberCube Object Reference"))
  (bind _asbp_number_cube (cast `/Game/Blueprint/BP_NumberCube` (`|GetArrayItem` (`PrimitiveComponent.GetOverlappingActors` (`self.Box`) "/Game/Blueprint/BP_NumberCube.BP_NumberCube_C"))))
  (return _asbp_number_cube))